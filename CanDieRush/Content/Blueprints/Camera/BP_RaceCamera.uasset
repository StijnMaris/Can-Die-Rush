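; Race camera that tracks players and switches every player controller's view between itself and two end cameras near the finish.
; While tracking, Tick compares its distance to EndPoint against two threshold points, with DoOnce gates firing each eased view blend once per zone change.
; A winner or all players dead ends the race and blends views back to this camera until Reset clears both flags.
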(event EventBeginPlay
  ;[1 1 1] Initialisation
  (bind _outactors (Actor|GetAllActorsOfClass "/Script/CanDieRush.RacePlayerController"))
  (Variables|Default|SetPlayerControllers _outactors)
  (Class|RaceCameraActor|SetGoal "0, 0, 0"))

(event Collision|EventActorBeginOverlap
  (params (OtherActor :type Actor%20Object%20Reference)))

(event EventTick
  (params (DeltaSeconds :type Float%20%28single-precision%29))
  (bind _endpoint (Variables|Default|GetEndPoint))
  (bind _returnvalue (Transformation|GetDistanceTo _endpoint))
  ;[1 1 1] Switch To End Camera
  (bind _returnvalue_2 (Class|RaceCameraActor|IsTrackingPlayers))
  (if _returnvalue_2
    (if (not (Variables|Default|GetHasFinished))
      (Variables|Default|SetHasEveryoneDied true)
      (for _array_element (Variables|Default|GetPlayerControllers)
        (bind _asbp_race_character (Utilities|Casting|CastToBP_RaceCharacter (Pawn|GetControlledPawn _array_element)))
        (bind _returnvalue_3 (Class|RaceCharacter|GetHasWon _asbp_race_character))
        (Variables|Default|SetHasWinner (or _returnvalue_3 (Variables|Default|GetHasWinner)))
        (Variables|Default|SetHasEveryoneDied (and (Variables|/Game/Blueprints/Player/BP_RaceCharacter.BP_RaceCharacter_C|GetIsDead _asbp_race_character) (Variables|Default|GetHasEveryoneDied))))
      (if (or (Variables|Default|GetHasWinner) (Variables|Default|GetHasEveryoneDied))
        (Variables|Default|SetHasFinished true)
        (for _array_element_2 (Variables|Default|GetPlayerControllers) :!label _label
          (Game|Player|SetViewTargetwithBlend _array_element_2 self 2.0 "VTBlend_EaseIn" 1.0 false))
        (elif (< _returnvalue (Transformation|GetDistanceTo _endpoint (Variables|Default|GetStartEndPoint)))
          (if (< _returnvalue (Transformation|GetDistanceTo _endpoint (Variables|Default|GetStartEndPoint2)))
            (Utilities|FlowControl|Sequence
              (:then_0
                (goto _label_3 Reset))
              (:then_1
                (goto _label_4 Reset))
              (:then_2
                (Utilities|FlowControl|DoOnce false :!label _label_2
                  (:Completed
                    (for _array_element_3 (Variables|Default|GetPlayerControllers)
                      (Game|Player|SetViewTargetwithBlend _array_element_3 (Variables|Default|GetEndCamera2) 2.0 "VTBlend_EaseOut" 1.0 false))))))
            (else
              (Utilities|FlowControl|Sequence
                (:then_0
                  (goto _label_4 Reset))
                (:then_1
                  (goto _label_2 Reset))
                (:then_2
                  (Utilities|FlowControl|DoOnce false :!label _label_3
                    (:Completed
                      (for _array_element_4 (Variables|Default|GetPlayerControllers)
                        (Game|Player|SetViewTargetwithBlend _array_element_4 (Variables|Default|GetEndCamera) 2.0 "VTBlend_EaseOut" 1.0 false))))))))
          (else
            (Utilities|FlowControl|Sequence
              (:then_0
                (goto _label_3 Reset))
              (:then_1
                (goto _label_2 Reset))
              (:then_2
                (Utilities|FlowControl|DoOnce false :!label _label_4
                  (:Completed
                    (goto _label)))))))))))

(fn ConstructionScript)

(fn Reset
  (Variables|Default|SetHasFinished false)
  (Variables|Default|SetHasWinner false))