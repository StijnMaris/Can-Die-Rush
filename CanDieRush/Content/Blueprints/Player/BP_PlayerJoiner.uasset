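; BP_PlayerJoiner lets one player slot join the game with the Jump action, leading into character selection.
; On press it disables its input, increments the game mode's player count and spawns a BP_SelectCharacter at the slot's tagged actor.
; The slot's controller possesses and initialises that character and is set active, while player 0's view switches to the selection camera.
; Helper functions enable or disable the slot's input.
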(event EventBeginPlay)

(event Collision|EventActorBeginOverlap
  (params (OtherActor :type Actor%20Object%20Reference)))

(event EventTick
  (params (DeltaSeconds :type Float%20%28single-precision%29)))

(event Input|ActionEvents|InputActionJump
  (params (Key :type Key%20Structure))
  (bind _player (Variables|Default|GetPlayer))
  (bind _returnvalue (Game|GetPlayerController _player))
  (:Pressed
    (Input|DisableInput (Game|GetPlayerController (Variables|Default|GetPlayer)))
    (bind _asbp_can_die_rush_game_mode (Utilities|Casting|CastToBP_CanDieRushGameMode (Game|GetGameMode)))
    (Variables|/Game/Blueprints/GameModes/BP_CanDieRushGameMode.BP_CanDieRushGameMode_C|SetAmountOfplayers _asbp_can_die_rush_game_mode (+ (Variables|/Game/Blueprints/GameModes/BP_CanDieRushGameMode.BP_CanDieRushGameMode_C|GetAmountOfplayers _asbp_can_die_rush_game_mode) 1))
    (bind _outactors (Actor|GetAllActorswithTag (Utilities|String|StringToName (Utilities|String|Append (Utilities|String|MakeLiteralString "Player") (Utilities|String|ToString(Integer) (Variables|Default|GetPlayer))))))
    (bind _returnvalue_2 (Game|SpawnActorfromClass "/Game/Blueprints/Player/BP_SelectCharacter.BP_SelectCharacter_C" (Transformation|GetActorTransform (Utilities|Array|Get(acopy) _outactors)) "Undefined" 0 0))
    (Pawn|Possess _returnvalue _returnvalue_2)
    (Class|RaceCharacter|SetPlayerID _returnvalue_2 (Variables|Default|GetPlayer))
    (Default|SetPlayerNameUI _returnvalue_2)
    (Default|SetPlayerCharacter _returnvalue_2)
    (bind _asrace_player_controller (Utilities|Casting|CastToRacePlayerController _returnvalue))
    (Class|RacePlayerController|SetActiveState _asrace_player_controller true)
    (bind _outactors_2 (Actor|GetAllActorsOfClass "/Game/Blueprints/Camera/BP_CharacterSelectCamera.BP_CharacterSelectCamera_C"))
    (Game|Player|SetViewTargetwithBlend (Game|GetPlayerController 0) (Utilities|Array|Get(acopy) _outactors_2) 0.0 "VTBlend_Linear" 0.0 false)))

(fn ConstructionScript)

(fn EnableInput
  (Input|EnableInput (Game|GetPlayerController (Variables|Default|GetPlayer))))

(fn DisableInput
  (Input|DisableInput (Game|GetPlayerController (Variables|Default|GetPlayer))))