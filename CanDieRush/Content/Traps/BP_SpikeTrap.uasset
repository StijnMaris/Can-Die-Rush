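; BP_SpikeTrap is a spike trap that kills any BP_RaceCharacter overlapping its spikes.
; On BeginPlay, RandomTrapIndex selects one of three candy-themed looks by swapping meshes and materials on the base and spikes, with index 0 doubling as the default.
; The spike mesh's begin-overlap event casts the other actor to the race character and calls KillCharacter.
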(event OnComponentBeginOverlap(SpikesMesh)
  (params (OverlappedComponent :type Primitive%20Component%20Object%20Reference) (OtherActor :type Actor%20Object%20Reference) (OtherComp :type Primitive%20Component%20Object%20Reference) (OtherBodyIndex :type Integer) (bFromSweep :type Boolean) (SweepResult :type Hit%20Result%20Structure%20%28by%20ref%29))
  (bind _asbp_race_character (Utilities|Casting|CastToBP_RaceCharacter OtherActor))
  (Default|KillCharacter _asbp_race_character))

(event EventBeginPlay
  (bind _trapmesh (Variables|Default|GetTrapMesh))
  (bind _trapmesh_2 (Variables|Default|GetTrapMesh))
  (bind _spikesmesh (Variables|Default|GetSpikesMesh))
  (bind _spikesmesh_2 (Variables|Default|GetSpikesMesh))
  (switch int (Variables|Default|GetRandomTrapIndex)
    (:Default
      (Components|StaticMesh|SetStaticMesh _trapmesh_2 "/Game/art_assets/traps/Spikes/MS_Spikes_ondergrond_spekjes.MS_Spikes_ondergrond_spekjes" :!label _label)
      (Components|StaticMesh|SetStaticMesh _spikesmesh_2 "/Game/art_assets/traps/Spikes/MS_spikes_spekjes.MS_spikes_spekjes")
      (Rendering|Material|SetMaterial _trapmesh 0 "/Game/art_assets/traps/Spikes/Inst_spike_trap_spekjes.Inst_spike_trap_spekjes")
      (Rendering|Material|SetMaterial _spikesmesh 0 0))
    (:0
      (goto _label))
    (:1
      (Components|StaticMesh|SetStaticMesh _trapmesh_2 "/Game/art_assets/traps/Spikes/MS_Spikes_ondergrond_koekje.MS_Spikes_ondergrond_koekje")
      (Components|StaticMesh|SetStaticMesh _spikesmesh_2 "/Game/art_assets/traps/Spikes/MS_spikes_ice_cream.MS_spikes_ice_cream")
      (Rendering|Material|SetMaterial _trapmesh 0 "/Game/art_assets/traps/Spikes/Inst_spike_trap_ice_cream.Inst_spike_trap_ice_cream")
      (Rendering|Material|SetMaterial _spikesmesh 0 "/Game/art_assets/traps/Spikes/Inst_spike_trap_ice_cream.Inst_spike_trap_ice_cream"))
    (:2
      (Components|StaticMesh|SetStaticMesh _trapmesh_2 "/Game/art_assets/traps/Spikes/MS_Spikes__ondergrondchocolate.MS_Spikes__ondergrondchocolate")
      (Components|StaticMesh|SetStaticMesh _spikesmesh_2 "/Game/art_assets/traps/Spikes/MS_spikes_candy_cane.MS_spikes_candy_cane")
      (Rendering|Material|SetMaterial _trapmesh 0 "/Game/art_assets/traps/Spikes/Inst_spike_trap_ice_candy_cane.Inst_spike_trap_ice_candy_cane")
      (Rendering|Material|SetMaterial _spikesmesh 0 "/Game/art_assets/traps/Spikes/Inst_spike_trap_ice_candy_cane.Inst_spike_trap_ice_candy_cane"))))

(event EventTick
  (params (DeltaSeconds :type Float%20%28single-precision%29)))

(fn ConstructionScript)