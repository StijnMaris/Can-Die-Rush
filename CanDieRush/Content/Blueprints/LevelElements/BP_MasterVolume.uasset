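; BP_MasterVolume is a level element whose mesh position shows the game's current master volume, like a slider handle.
; Each tick it casts the game mode to BP_CanDieRushGameMode and sets the mesh's relative X to MasterVolume times a fixed travel distance, without sweeping.
; It only reads the volume and never changes it.
; The start location stored at BeginPlay is not used in these graphs.
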(event EventBeginPlay
  (Variables|Default|SetStartLocation (Transformation|GetWorldLocation (Variables|Default|GetStaticMesh))))

(event Collision|EventActorBeginOverlap
  (params (OtherActor :type Actor%20Object%20Reference)))

(event EventTick
  (params (DeltaSeconds :type Float%20%28single-precision%29))
  (bind _asbp_can_die_rush_game_mode (Utilities|Casting|CastToBP_CanDieRushGameMode (Game|GetGameMode)))
  (Transformation|SetRelativeLocation (Variables|Default|GetStaticMesh) (Math|Vector|MakeVector (* (Variables|/Game/Blueprints/GameModes/BP_CanDieRushGameMode.BP_CanDieRushGameMode_C|GetMaster%20Volume _asbp_can_die_rush_game_mode) 168.0) 0.0 0.0) false false))

(fn ConstructionScript)