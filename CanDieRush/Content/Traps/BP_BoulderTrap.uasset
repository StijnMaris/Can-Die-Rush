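; Boulder trap that enables physics on a destructible boulder when its trigger box is overlapped.
; An unfractured boulder hitting a BP_RaceCharacter takes impact damage and kills the character.
; First impact spawns brief dust and a sound; fracturing sets the harmless state and plays the sound, scaled by game-mode master volume.
; ResetBoulderTrap restores the mesh, disables physics and repositions it at BoulderMesh, leaving the Hit and Fractured flags unchanged.
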(event OnComponentFracture(SM_boulder_full_DM)
  (params (HitPoint :type Vector%20%28by%20ref%29 :default "0, 0, 0") (HitDirection :type Vector%20%28by%20ref%29 :default "0, 0, 0"))
  (Variables|Default|SetFractured true)
  (bind _asbp_can_die_rush_game_mode (Utilities|Casting|CastToBP_CanDieRushGameMode (Game|GetGameMode)))
  (Audio|SpawnSound2D "/Game/art_assets/SoundEffects/Boulder_Cue.Boulder_Cue" (Math|Float|Clamp(Float) (Variables|/Game/Blueprints/GameModes/BP_CanDieRushGameMode.BP_CanDieRushGameMode_C|GetMaster%20Volume _asbp_can_die_rush_game_mode) "0.01f" (Variables|/Game/Blueprints/GameModes/BP_CanDieRushGameMode.BP_CanDieRushGameMode_C|GetMaster%20Volume _asbp_can_die_rush_game_mode))))

(event OnComponentHit(boulder_full_DM1)
  (params (HitComponent :type Primitive%20Component%20Object%20Reference) (OtherActor :type Actor%20Object%20Reference) (OtherComp :type Primitive%20Component%20Object%20Reference) (NormalImpulse :type Vector :default "0, 0, 0") (Hit :type Hit%20Result%20Structure%20%28by%20ref%29))
  (bind (_bblockinghit _binitialoverlap _time _distance _location _impactpoint _normal _impactnormal) (Collision|BreakHitResult Hit))
  (Utilities|FlowControl|Sequence
    (:then_0
      (if (Variables|Default|GetFractured)
        (Development|PrintString "branch fail" false false)
        (else
          (bind _asbp_race_character (Utilities|Casting|CastToBP_RaceCharacter OtherActor))
          (Class|DestructibleComponent|ApplyDamage (Variables|Default|Getboulder_full_DM1) 15.0 _impactpoint _impactnormal 1e+03)
          (Development|PrintString "kill")
          (Default|KillCharacter _asbp_race_character))))
    (:then_1
      (if (not (Variables|Default|GetHit))
        (bind _returnvalue (Effects|SpawnEmitteratLocation "/Game/particles/boulder/PS_impactDust.PS_impactDust" (+ _location "0, 0,10.000000") "0, 0, 0" "2.000000,2.000000,2.000000"))
        (Variables|Default|SetHit true)
        (bind _asbp_can_die_rush_game_mode (Utilities|Casting|CastToBP_CanDieRushGameMode (Game|GetGameMode)))
        (Audio|SpawnSound2D "/Game/art_assets/SoundEffects/Boulder_Cue.Boulder_Cue" (Math|Float|Clamp(Float) (Variables|/Game/Blueprints/GameModes/BP_CanDieRushGameMode.BP_CanDieRushGameMode_C|GetMaster%20Volume _asbp_can_die_rush_game_mode) "0.01f" (Variables|/Game/Blueprints/GameModes/BP_CanDieRushGameMode.BP_CanDieRushGameMode_C|GetMaster%20Volume _asbp_can_die_rush_game_mode)))
        (Utilities|FlowControl|Delay 1.0)
        (Components|DestroyComponent _returnvalue)))))

(event OnComponentBeginOverlap(TriggerBox)
  (params (OverlappedComponent :type Primitive%20Component%20Object%20Reference) (OtherActor :type Actor%20Object%20Reference) (OtherComp :type Primitive%20Component%20Object%20Reference) (OtherBodyIndex :type Integer) (bFromSweep :type Boolean) (SweepResult :type Hit%20Result%20Structure%20%28by%20ref%29))
  (Physics|SetSimulatePhysics (Variables|Default|Getboulder_full_DM1) true))

(event EventBeginPlay)

(event Collision|EventActorBeginOverlap
  (params (OtherActor :type Actor%20Object%20Reference)))

(event EventTick
  (params (DeltaSeconds :type Float%20%28single-precision%29)))

(fn ConstructionScript)

(fn ResetBoulderTrap
  (bind _boulder_full_dm1 (Variables|Default|Getboulder_full_DM1))
  (Class|DestructibleComponent|SetDestructibleMesh _boulder_full_dm1 "/Game/art_assets/traps/boulder/boulder_full_DM.boulder_full_DM")
  (Physics|SetSimulatePhysics _boulder_full_dm1 false)
  (Transformation|SetWorldLocation (Variables|Default|Getboulder_full_DM1) (Transformation|GetWorldLocation (Variables|Default|GetBoulderMesh)) false false))