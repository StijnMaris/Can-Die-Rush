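; BP_EndCharacterSelect is a trigger zone that ends character selection and starts the building phase.
; Box overlaps keep a count of the BP_SelectCharacter actors standing inside.
; Tick waits until that count is at least two and equals the game mode's player count, then fires once.
; A timeline acts as a delay, then calls StartBuilding on BP_CanDieRushGameMode and removes every select character's UI.
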(event OnComponentBeginOverlap(Box)
  (params (OverlappedComponent :type Primitive%20Component%20Object%20Reference) (OtherActor :type Actor%20Object%20Reference) (OtherComp :type Primitive%20Component%20Object%20Reference) (OtherBodyIndex :type Integer) (bFromSweep :type Boolean) (SweepResult :type Hit%20Result%20Structure%20%28by%20ref%29))
  (Utilities|Casting|CastToBP_SelectCharacter OtherActor)
  (bind _output_get (Variables|Default|SetReadyPlayers (+ (Variables|Default|GetReadyPlayers) 1))))

(event OnComponentEndOverlap(Box)
  (params (OverlappedComponent :type Primitive%20Component%20Object%20Reference) (OtherActor :type Actor%20Object%20Reference) (OtherComp :type Primitive%20Component%20Object%20Reference) (OtherBodyIndex :type Integer))
  (Utilities|Casting|CastToBP_SelectCharacter OtherActor)
  (bind _output_get (Variables|Default|SetReadyPlayers (+ (Variables|Default|GetReadyPlayers) -1))))

(event EventBeginPlay)

(event Collision|EventActorBeginOverlap
  (params (OtherActor :type Actor%20Object%20Reference)))

(event EventTick
  (params (DeltaSeconds :type Float%20%28single-precision%29))
  (bind _readyplayers (Variables|Default|GetReadyPlayers))
  (bind _asbp_can_die_rush_game_mode (Utilities|Casting|CastToBP_CanDieRushGameMode (Game|GetGameMode)))
  (if (Math|Boolean|ANDBoolean (>= _readyplayers 2) (== _readyplayers (Variables|/Game/Blueprints/GameModes/BP_CanDieRushGameMode.BP_CanDieRushGameMode_C|GetAmountOfplayers _asbp_can_die_rush_game_mode)) (not (Variables|Default|GetHasActived)))
    (Variables|Default|SetHasActived true)
    (Development|PrintString "Start building")
    (Timeline|Timeline_0 PlayFromStart
      (:Finished
        (Default|StartBuilding _asbp_can_die_rush_game_mode)
        (bind _outactors (Actor|GetAllActorsOfClass "/Game/Blueprints/Player/BP_SelectCharacter.BP_SelectCharacter_C"))
        (for _array_element _outactors
          (Default|RemoveUI _array_element))))))

(fn ConstructionScript)