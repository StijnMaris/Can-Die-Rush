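; Game mode for the local multiplayer Can Die Rush, cycling players through trap-building and racing phases and back to the menu.
; Tick watches surviving race characters, flags the last one as winner, then starts building behind a fade cinematic.
; Each phase respawns or repossesses character and building pawns per player controller, hands them to its camera and uses a countdown timeline.
; It also owns the HUD and switches menu and race music.
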(event Custom|Start%20Building
  (bind _builingfade (Variables|Default|GetBuilingFade))
  (bind _sequenceplayer (Variables|/Script/LevelSequence.LevelSequenceActor|GetSequencePlayer _builingfade))
  (Utilities|FlowControl|DoOnce false :!label _label
    (:Completed
      (Class|MovieSceneSequencePlayer|JumptoPosition _sequenceplayer 0.0)
      (Sequencer|Player|Play _sequenceplayer :!class /Script/MovieScene.MovieSceneSequencePlayer)
      (Variables|Default|SetIsBuilding true)
      (Utilities|FlowControl|Delay 0.4175)
      (CallFunction|SetupBuilding)
      (bind _stuff (Timeline|Building%20waiting PlayFromStart)
        (:Update
          (bind _output_get (Variables|Default|SetCurrentTime _stuff))
          (if (<= _output_get 0.0)
            (Utilities|FlowControl|DoOnce false :!label _label_2
              (:Completed
                (bind _outactors (Actor|GetAllActorsOfClass "/Game/Blueprints/Camera/BP_BuildingCamera.BP_BuildingCamera_C"))
                (for _array_element _outactors
                  (Class|BuildingCameraActor|StartBuildMode _array_element)
                  (Variables|/Game/Blueprints/Camera/BP_BuildingCamera.BP_BuildingCamera_C|SetIsActive _array_element true)
                  (Variables|/Game/Blueprints/Camera/BP_BuildingCamera.BP_BuildingCamera_C|SetDoSkipBuilding _array_element false)
                  (Variables|Default|SetIsInCharacterSelect false)
                  (goto _label Reset))))))
        (:Finished
          (goto _label_2 Reset))))))

(event Custom|Change%20Volume
  (Audio|Components|Audio|AdjustVolume (Variables|Default|GetBackGroundMusic) 0.0 (Math|Float|Clamp(Float) (Variables|Default|GetSound%20Volume) "0.01f" (Variables|Default|GetMaster%20Volume)) :!class /Script/Engine.AudioComponent))

(event Custom|Start%20Racing%20Event
  (CallFunction|SetupRacing)
  (Variables|Default|SetIsBuilding false)
  (bind _stuff (Timeline|Racing%20Waiting PlayFromStart)
    (:Update
      (bind _output_get (Variables|Default|SetCurrentTime _stuff))
      (if (<= _output_get 0.0)
        (Utilities|FlowControl|DoOnce false :!label _label
          (:Completed
            (CallFunction|StartRacing)))))
    (:Finished
      (goto _label Reset))))

(event EventTick
  (params (DeltaSeconds :type Float%20%28single-precision%29))
  (if (not (Variables|Default|GetIsInCharacterSelect))
    (bind _outactors (Actor|GetAllActorsOfClass "/Game/Blueprints/Player/BP_RaceCharacter.BP_RaceCharacter_C"))
    (if (not (> (Utilities|Array|Length _outactors) 1))
      (if (!= (Variables|Default|GetAmountOfplayers) 1)
        (for _array_element _outactors
          (if (not (Variables|/Game/Blueprints/Player/BP_RaceCharacter.BP_RaceCharacter_C|GetIsDead _array_element))
            (Class|RaceCharacter|SetHasWon _array_element)))
        (Utilities|FlowControl|Delay 2.0 :!label _label)
        (CallFunction|StartBuilding)
        (elif (not (> (Utilities|Array|Length _outactors) 0))
          (goto _label))))))

(event EventBeginPlay
  (bind _returnvalue (UserInterface|CreateWidget "/Game/UI/UIBP_RaceHud.UIBP_RaceHud_C"))
  (UserInterface|Viewport|AddtoViewport _returnvalue 5)
  (bind _outactors (Actor|GetAllActorsOfClass "/Game/Blueprints/Player/BP_PlayerSpawn.BP_PlayerSpawn_C"))
  (Variables|Default|SetPlayerSpawns _outactors)
  (bind _returnvalue_2 (Audio|SpawnSound2D "/Game/art_assets/Music/Menu_Music_Cue.Menu_Music_Cue" (Math|Float|Clamp(Float) (Variables|Default|GetSound%20Volume) "0.01f" (Variables|Default|GetMaster%20Volume))))
  (Variables|Default|SetBackGroundMusic _returnvalue_2)
  ;[1 1 1] Set cinematic
  (bind _outactors_2 (Actor|GetAllActorsOfClass "/Script/LevelSequence.LevelSequenceActor"))
  (for _array_element _outactors_2
    (if (Utilities|Enum|Equal(Enum) (Utilities|GetObjectName _array_element) "StartBuildingCinematic")
      (Variables|Default|SetBuilingFade _array_element)
      (Development|PrintString "Animation Set"))))

(fn ConstructionScript)

(fn SetupBuilding
  (if (== (Variables|/Script/Engine.AudioComponent|GetSound (Variables|Default|GetBackGroundMusic)) "/Game/art_assets/Music/Menu_Music_Cue.Menu_Music_Cue")
    _
    (else
      (Audio|Components|Audio|Stop (Variables|Default|GetBackGroundMusic))
      (bind _returnvalue (Audio|SpawnSound2D "/Game/art_assets/Music/Menu_Music_Cue.Menu_Music_Cue" (Math|Float|Clamp(Float) (Variables|Default|GetSound%20Volume) "0.01f" (Variables|Default|GetMaster%20Volume))))
      (Variables|Default|SetBackGroundMusic _returnvalue)
      (bind _outactors (Actor|GetAllActorsOfClass "/Game/Traps/BP_BoulderTrap.BP_BoulderTrap_C"))
      (for _array_element _outactors
        (Default|ResetBoulderTrap _array_element))))
  ;[1 1 1] Destroy all remaining players
  (bind _outactors_2 (Actor|GetAllActorsOfClass "/Game/Blueprints/Player/BP_RaceCharacter.BP_RaceCharacter_C"))
  (for _array_element_2 _outactors_2
    (Actor|DestroyActor _array_element_2))
  (bind _outactors_3 (Actor|GetAllActorsOfClass "/Game/Blueprints/Player/BP_BuildingPawn.BP_BuildingPawn_C"))
  (for _array_element_3 _outactors_3
    (Actor|DestroyActor _array_element_3))
  ;[1 1 1] Spawning race characters
  (for _index (range 0 (- (Variables|Default|GetAmountOfplayers) 1))
    (bind _returnvalue_2 (Game|SpawnActorfromClass "/Game/Blueprints/Player/BP_RaceCharacter.BP_RaceCharacter_C" (Transformation|GetActorTransform (Utilities|Array|Get(acopy) (Variables|Default|GetPlayerSpawns) _index)) "Undefined" 0 0))
    (bind _asrace_player_controller (Utilities|Casting|CastToRacePlayerController (Game|GetPlayerController _index)))
    (bind _returnvalue_3 (Class|RacePlayerController|GetCharacterId _asrace_player_controller))
    (Class|RaceCharacter|SetPlayerID _returnvalue_2 _index)
    (Pawn|Possess (Game|GetPlayerController _index) _returnvalue_2)
    (Default|SetPlayerNameUI _returnvalue_2)
    (Default|SetPlayerCharacter _returnvalue_2 _returnvalue_3))
  (bind _outactors_4 (Actor|GetAllActorsOfClass "/Game/Blueprints/Camera/BP_RaceCamera.BP_RaceCamera_C"))
  (for _array_element_4 _outactors_4
    (Class|RaceCameraActor|SetGoal _array_element_4 "0, 0, 0"))
  ;[1 1 1] Camera
  (bind _outactors_5 (Actor|GetAllActorsOfClass "/Game/Blueprints/Player/BP_RaceCharacter.BP_RaceCharacter_C"))
  (bind _outactors_6 (Actor|GetAllActorsOfClass "/Game/Blueprints/Camera/BP_BuildingCamera.BP_BuildingCamera_C"))
  (for _array_element_5 _outactors_6
    (Class|BuildingCameraActor|SetPlayers _array_element_5 _outactors_5)
    (CallFunction|SetupBuildingPawn)
    (Class|BuildingCameraActor|PrepareBuildingMode _array_element_5)))

(fn SetupBuildingPawn
  (for _index (range 0 (- (Variables|Default|GetAmountOfplayers) 1))
    (LocalVariables|SetPlayerIndex _index)
    (LocalVariables|SetPlayerController (Game|GetPlayerController (LocalVariables|GetPlayerIndex)))
    (Utilities|Casting|CastToRaceCharacter (Pawn|GetControlledPawn (LocalVariables|GetPlayerController)))
    (Development|PrintString (Utilities|String|Append (Utilities|String|MakeLiteralString "Set Player id: ") (Utilities|String|ToString(Integer) (LocalVariables|GetPlayerIndex))))
    (bind _outactors (Actor|GetAllActorsOfClass "/Game/Blueprints/Camera/BP_BuildingCamera.BP_BuildingCamera_C"))
    (bind _output_get (LocalVariables|SetBuildingCameras _outactors))
    (for _array_element _output_get
      (bind _output_get_2 (Variables|Default|SetStartTransform (Transformation|GetActorTransform _array_element)))
      (bind _returnvalue (Game|SpawnActorfromClass "/Game/Blueprints/Player/BP_BuildingPawn.BP_BuildingPawn_C" (Math|Transform|MakeTransform (Math|Vector|MakeVector (+ (.X (Math|Vector|BreakVector (.Location (Math|Transform|BreakTransform _output_get_2)))) -1e+03) (+ (- (.Y (Math|Vector|BreakVector (.Location (Math|Transform|BreakTransform _output_get_2)))) 2e+02) (* (LocalVariables|GetPlayerIndex) 2e+02)) 0.0)) "Undefined" 0 0))
      (Class|BuildingPawn|SetSpawnLocation _returnvalue (Math|Vector|MakeVector (+ (.X (Math|Vector|BreakVector (.Location (Math|Transform|BreakTransform _output_get_2)))) -1e+03) (+ (- (.Y (Math|Vector|BreakVector (.Location (Math|Transform|BreakTransform _output_get_2)))) 2e+02) (* (LocalVariables|GetPlayerIndex) 2e+02)) 0.0))
      (Pawn|Possess (LocalVariables|GetPlayerController) _returnvalue)
      (Default|SetPawnColorfromController _returnvalue))
    (for _array_element_2 (LocalVariables|GetBuildingCameras)
      (Transformation|SetActorLocation _array_element_2 (Variables|/Script/CanDieRush.BuildingCameraActor|GetStart _array_element_2) false true))))

(fn SetupRacing
  (bind _master_volume (Variables|Default|GetMaster%20Volume))
  (Audio|Components|Audio|Stop (Variables|Default|GetBackGroundMusic))
  (Utilities|FlowControl|Sequence
    (:then_0
      (Audio|SpawnSound2D "/Game/art_assets/SoundEffects/Go_Cue.Go_Cue" (Math|Float|Clamp(Float) _master_volume 0.01 _master_volume))
      (bind _outactors (Actor|GetAllActorsOfClass "/Game/Blueprints/Player/BP_RaceCharacter.BP_RaceCharacter_C"))
      (for _array_element _outactors
        (bind _returnvalue (Class|RaceCharacter|GetPlayerID _array_element))
        (Pawn|Possess (Game|GetPlayerController _returnvalue) _array_element)
        (Input|DisableInput _array_element (Game|GetPlayerController _returnvalue))
        (Default|SetPlayerNameUI _array_element))
      (bind _outactors_2 (Actor|GetAllActorsOfClass "/Game/Blueprints/Camera/BP_RaceCamera.BP_RaceCamera_C"))
      (for _array_element_2 _outactors_2
        (Class|RaceCameraActor|SetPlayers _array_element_2 _outactors)
        (Class|RaceCameraActor|StartRaceMode _array_element_2)
        (Development|PrintText "Starting Racemode"))
      (Development|PrintText "Done looking for RaceCamera's"))))

(fn StartRacing
  (Utilities|FlowControl|Sequence
    (:then_0
      (bind _outactors (Actor|GetAllActorsOfClass "/Game/Blueprints/Camera/BP_RaceCamera.BP_RaceCamera_C"))
      (for _array_element _outactors
        (Default|Reset _array_element)))
    (:then_1
      (bind _returnvalue (Audio|SpawnSound2D "/Game/art_assets/Music/Race_Music_Cue.Race_Music_Cue" (Math|Float|Clamp(Float) (Variables|Default|GetSound%20Volume) "0.01f" (Variables|Default|GetMaster%20Volume))))
      (Variables|Default|SetBackGroundMusic _returnvalue)
      (bind _outactors_2 (Actor|GetAllActorsOfClass "/Game/Blueprints/Player/BP_RaceCharacter.BP_RaceCharacter_C"))
      (for _array_element_2 _outactors_2
        (bind _returnvalue_2 (Class|RaceCharacter|GetPlayerID _array_element_2))
        (Input|EnableInput _array_element_2 (Game|GetPlayerController _returnvalue_2))
        (Default|SetPlayerNameUI _array_element_2)))))

(fn ResettoMenu
  (bind _returnvalue (Game|GetPlayerController 0))
  (Variables|Default|SetIsInCharacterSelect true)
  ;[1 1 1] Destroy all remaining players and traps
  (bind _outactors (Actor|GetAllActorsOfClass "/Game/Blueprints/Player/BP_RaceCharacter.BP_RaceCharacter_C"))
  (for _array_element _outactors
    (Actor|DestroyActor _array_element))
  (bind _outactors_2 (Actor|GetAllActorsOfClass "/Game/Blueprints/Player/BP_BuildingPawn.BP_BuildingPawn_C"))
  (for _array_element_2 _outactors_2
    (Actor|DestroyActor _array_element_2))
  (bind _outactors_3 (Actor|GetAllActorsOfClass "/Game/Blueprints/Player/BP_SelectCharacter.BP_SelectCharacter_C"))
  (for _array_element_3 _outactors_3
    (Actor|DestroyActor _array_element_3))
  (bind _outactors_4 (Actor|GetAllActorsOfClass "/Script/CanDieRush.LethalTrap"))
  (for _array_element_4 _outactors_4
    (Actor|DestroyActor _array_element_4))
  (bind _outactors_5 (Actor|GetAllActorsOfClass "/Script/CanDieRush.RacePlayerController"))
  (for _array_element_5 _outactors_5
    (Class|RacePlayerController|Reset _array_element_5))
  (Variables|Default|SetAmountOfplayers 0)
  (Variables|Default|SetIsBuilding false)
  ;[1 1 1] MenuCamera
  (bind _outactors_6 (Actor|GetAllActorsOfClass "/Game/Blueprints/Camera/BP_MenuCamera.BP_MenuCamera_C"))
  (for _array_element_6 _outactors_6
    (Input|EnableInput _array_element_6 _returnvalue)
    (Game|Player|SetViewTargetwithBlend _returnvalue _array_element_6 0.0 "VTBlend_Linear" 0.0 false))
  (if (== (Variables|/Script/Engine.AudioComponent|GetSound (Variables|Default|GetBackGroundMusic)) "/Game/art_assets/Music/Menu_Music_Cue.Menu_Music_Cue")
    _
    (else
      (Audio|Components|Audio|Stop (Variables|Default|GetBackGroundMusic))
      (bind _returnvalue_2 (Audio|SpawnSound2D "/Game/art_assets/Music/Menu_Music_Cue.Menu_Music_Cue" (Math|Float|Clamp(Float) (Variables|Default|GetSound%20Volume) "0.01f" (Variables|Default|GetMaster%20Volume))))
      (Variables|Default|SetBackGroundMusic _returnvalue_2)))
  ;[1 1 1] PlayerJoiners
  (bind _outactors_7 (Actor|GetAllActorsOfClass "/Game/Blueprints/Player/BP_PlayerJoiner.BP_PlayerJoiner_C"))
  (for _array_element_7 _outactors_7
    (Default|DisableInput _array_element_7))
  ;[1 1 1] Building camera
  (bind _outactors_8 (Actor|GetAllActorsOfClass "/Game/Blueprints/Camera/BP_BuildingCamera.BP_BuildingCamera_C"))
  (for _array_element_8 _outactors_8
    (Variables|/Game/Blueprints/Camera/BP_BuildingCamera.BP_BuildingCamera_C|SetIsActive _array_element_8 false))
  ;[1 1 1] RaceCamera
  (bind _outactors_9 (Actor|GetAllActorsOfClass "/Game/Blueprints/Camera/BP_RaceCamera.BP_RaceCamera_C"))
  (for _array_element_9 _outactors_9
    (Class|RaceCameraActor|SetGoal _array_element_9 "0, 0, 0")))