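; Main menu camera for CanDieRush that takes player view and input and runs menu navigation, volume options, quit, and handoff to character selection.
; Highlights entries by swapping mask textures on dynamic materials applied to tagged meshes.
; Level sequences play forward and backward between screens, while volume changes go to BP_CanDieRushGameMode.
; Tick records the transform during menu sequences and reapplies it once they stop, as a position fix.
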(event EventBeginPlay
  (bind _returnvalue (Transformation|GetActorTransform))
  (bind _returnvalue_2 (Game|GetPlayerController 0))
  (bind (_location _rotation _scale) (Math|Transform|BreakTransform _returnvalue))
  (bind (_x _y _z) (Math|Vector|BreakVector _location))
  (Utilities|FlowControl|Sequence
    (:then_0
      (Input|EnableInput _returnvalue_2)
      (Game|Player|SetViewTargetwithBlend _returnvalue_2 self 0.0 "VTBlend_Linear" 0.0 false)
      (Variables|Default|SetCurrentTransform (Math|Transform|MakeTransform (Math|Vector|MakeVector _x (+ _y 1.4e+02) _z) _rotation _scale))
      (bind _returnvalue_3 (Rendering|Material|CreateDynamicMaterialInstance "/Game/art_assets/Startup_screen/M_Menu.M_Menu" :!class /Script/Engine.KismetMaterialLibrary))
      (Variables|Default|SetMaterial%20Menu _returnvalue_3)
      (bind _outactors (Actor|GetAllActorswithTag "Menu"))
      (for _array_element _outactors
        (if (Utilities|IsValid (Actor|GetComponentbyClass _array_element "/Script/Engine.StaticMeshComponent"))
          (Rendering|Material|SetMaterial (Actor|GetComponentbyClass _array_element "/Script/Engine.StaticMeshComponent") 0 (Variables|Default|GetMaterial%20Menu))
          (Development|PrintString "Material Set"))))
    (:then_1
      (bind _returnvalue_4 (Rendering|Material|CreateDynamicMaterialInstance "/Game/art_assets/Startup_screen/M_Option_inst.M_Option_inst" :!class /Script/Engine.KismetMaterialLibrary))
      (Variables|Default|SetMaterial%20OptionsMenu _returnvalue_4)
      (bind _outactors_2 (Actor|GetAllActorswithTag "OptionsMenu"))
      (for _array_element_2 _outactors_2
        (if (Utilities|IsValid (Actor|GetComponentbyClass _array_element_2 "/Script/Engine.StaticMeshComponent"))
          (Rendering|Material|SetMaterial (Actor|GetComponentbyClass _array_element_2 "/Script/Engine.StaticMeshComponent") 0 (Variables|Default|GetMaterial%20OptionsMenu))
          (Development|PrintString "Material Set"))))
    (:then_2
      (Sequencer|Player|Play (Variables|/Script/LevelSequence.LevelSequenceActor|GetSequencePlayer (Variables|Default|GetCinematicsToMenu)) :!class /Script/MovieScene.MovieSceneSequencePlayer))))

(event Collision|EventActorBeginOverlap
  (params (OtherActor :type Actor%20Object%20Reference)))

(event EventTick
  (params (DeltaSeconds :type Float%20%28single-precision%29))
  ;[1 1 1] Position fix
  (if (Math|Boolean|ORBoolean (Audio|Components|Audio|IsPlaying (Variables|/Script/LevelSequence.LevelSequenceActor|GetSequencePlayer (Variables|Default|GetCinematicToControls))) (Audio|Components|Audio|IsPlaying (Variables|/Script/LevelSequence.LevelSequenceActor|GetSequencePlayer (Variables|Default|GetCinematicsToMenu))) (Audio|Components|Audio|IsPlaying (Variables|/Script/LevelSequence.LevelSequenceActor|GetSequencePlayer (Variables|Default|GetCinematiccToOptions))))
    (Variables|Default|SetCurrentTransform (Transformation|GetActorTransform self))
    (goto _label Reset)
    (else
      (Utilities|FlowControl|DoOnce false :!label _label
        (:Completed
          (Transformation|SetActorTransform (Variables|Default|GetCurrentTransform)))))))

(event Input|ActionEvents|InputActionUpMenu
  (params (Key :type Key%20Structure))
  (bind _material_optionsmenu (Variables|Default|GetMaterial%20OptionsMenu))
  (bind _material_menu (Variables|Default|GetMaterial%20Menu))
  ;[1 1 1] MenuOption up and down
  (:Pressed
    (if (Variables|Default|GetIsInMainMenu)
      (Variables|Default|SetCurrentMenuOption (Math|Integer|%(Integer) (+ (Variables|Default|GetCurrentMenuOption) 3) 4))
      (switch int (Variables|Default|GetCurrentMenuOption)
        (:0
          (Rendering|Material|SetTextureParameterValue _material_menu "Mask" "/Game/UI/tex_startButtonMask.tex_startButtonMask"))
        (:1
          (Rendering|Material|SetTextureParameterValue _material_menu "Mask" "/Game/UI/tex_controlsButtonMask.tex_controlsButtonMask")
          (bind _asbp_can_die_rush_game_mode (Utilities|Casting|CastToBP_CanDieRushGameMode (Game|GetGameMode) :!label _label))
          (Audio|SpawnSound2D "/Game/art_assets/SoundEffects/BlackBoard.BlackBoard" (Math|Float|Clamp(Float) (Variables|/Game/Blueprints/GameModes/BP_CanDieRushGameMode.BP_CanDieRushGameMode_C|GetMaster%20Volume _asbp_can_die_rush_game_mode) "0.01f" (Variables|/Game/Blueprints/GameModes/BP_CanDieRushGameMode.BP_CanDieRushGameMode_C|GetMaster%20Volume _asbp_can_die_rush_game_mode))))
        (:2
          (Rendering|Material|SetTextureParameterValue _material_menu "Mask" "/Game/UI/tex_optionsButtonMask.tex_optionsButtonMask")
          (goto _label))
        (:3
          (Rendering|Material|SetTextureParameterValue _material_menu "Mask" "/Game/UI/tex_exitButtonMask.tex_exitButtonMask")))
      (elif (Variables|Default|GetIsInOption)
        (Variables|Default|SetCurrentOptionMenu (Math|Integer|%(Integer) (+ (Variables|Default|GetCurrentOptionMenu) 1) 2))
        (switch int (Variables|Default|GetCurrentOptionMenu)
          (:0
            (Rendering|Material|SetTextureParameterValue _material_optionsmenu "Mask" "/Game/art_assets/Startup_screen/Tex_master_volume_mask.Tex_master_volume_mask")
            (goto _label))
          (:1
            (Rendering|Material|SetTextureParameterValue _material_optionsmenu "Mask" "/Game/art_assets/Startup_screen/Tes_Music_mask.Tes_Music_mask")
            (goto _label)))))))

(event Input|ActionEvents|InputActionDownMenu
  (params (Key :type Key%20Structure))
  (bind _material_optionsmenu (Variables|Default|GetMaterial%20OptionsMenu))
  (bind _material_menu (Variables|Default|GetMaterial%20Menu))
  ;[1 1 1] MenuOption up and down
  (:Pressed
    (if (Variables|Default|GetIsInMainMenu)
      (Variables|Default|SetCurrentMenuOption (Math|Integer|%(Integer) (+ (Variables|Default|GetCurrentMenuOption) 1) 4))
      (switch int (Variables|Default|GetCurrentMenuOption)
        (:0
          (Rendering|Material|SetTextureParameterValue _material_menu "Mask" "/Game/UI/tex_startButtonMask.tex_startButtonMask"))
        (:1
          (Rendering|Material|SetTextureParameterValue _material_menu "Mask" "/Game/UI/tex_controlsButtonMask.tex_controlsButtonMask")
          (bind _asbp_can_die_rush_game_mode (Utilities|Casting|CastToBP_CanDieRushGameMode (Game|GetGameMode) :!label _label))
          (Audio|SpawnSound2D "/Game/art_assets/SoundEffects/BlackBoard.BlackBoard" (Math|Float|Clamp(Float) (Variables|/Game/Blueprints/GameModes/BP_CanDieRushGameMode.BP_CanDieRushGameMode_C|GetMaster%20Volume _asbp_can_die_rush_game_mode) "0.01f" (Variables|/Game/Blueprints/GameModes/BP_CanDieRushGameMode.BP_CanDieRushGameMode_C|GetMaster%20Volume _asbp_can_die_rush_game_mode))))
        (:2
          (Rendering|Material|SetTextureParameterValue _material_menu "Mask" "/Game/UI/tex_optionsButtonMask.tex_optionsButtonMask")
          (goto _label))
        (:3
          (Rendering|Material|SetTextureParameterValue _material_menu "Mask" "/Game/UI/tex_exitButtonMask.tex_exitButtonMask")))
      (elif (Variables|Default|GetIsInOption)
        (Variables|Default|SetCurrentOptionMenu (Math|Integer|%(Integer) (+ (Variables|Default|GetCurrentOptionMenu) 1) 2))
        (switch int (Variables|Default|GetCurrentOptionMenu)
          (:0
            (Rendering|Material|SetTextureParameterValue _material_optionsmenu "Mask" "/Game/art_assets/Startup_screen/Tex_master_volume_mask.Tex_master_volume_mask")
            (goto _label))
          (:1
            (Rendering|Material|SetTextureParameterValue _material_optionsmenu "Mask" "/Game/art_assets/Startup_screen/Tes_Music_mask.Tes_Music_mask")
            (goto _label)))))))

(event Input|ActionEvents|InputActionPush
  (params (Key :type Key%20Structure))
  ;[1 1 1] Back
  (:Pressed
    (if (Variables|Default|GetIsInMainMenu)
      (Class|MovieSceneSequencePlayer|PlayReverse (Variables|/Script/LevelSequence.LevelSequenceActor|GetSequencePlayer (Variables|Default|GetCinematicsToMenu)))
      (Variables|Default|SetHasToStart true)
      (else
        (switch int (Variables|Default|GetCurrentMenuOption)
          (:1
            (Variables|Default|SetIsInMainMenu true)
            (Class|MovieSceneSequencePlayer|PlayReverse (Variables|/Script/LevelSequence.LevelSequenceActor|GetSequencePlayer (Variables|Default|GetCinematicToControls))))
          (:2
            (Variables|Default|SetIsInMainMenu true)
            (Class|MovieSceneSequencePlayer|PlayReverse (Variables|/Script/LevelSequence.LevelSequenceActor|GetSequencePlayer (Variables|Default|GetCinematiccToOptions)))
            (Variables|Default|SetIsInOption false)))))))

(event Input|ActionEvents|InputActionJump
  (params (Key :type Key%20Structure))
  ;[1 1 1] Continue
  (:Pressed
    (if (Variables|Default|GetHasToStart)
      (Sequencer|Player|Play (Variables|/Script/LevelSequence.LevelSequenceActor|GetSequencePlayer (Variables|Default|GetCinematicsToMenu)) :!class /Script/MovieScene.MovieSceneSequencePlayer)
      (Variables|Default|SetHasToStart false)
      (else
        (switch int (Variables|Default|GetCurrentMenuOption)
          (:0
            (Input|DisableInput (Game|GetPlayerController 0))
            (bind _outactors (Actor|GetAllActorsOfClass "/Game/Blueprints/Player/BP_PlayerJoiner.BP_PlayerJoiner_C"))
            (for _array_element _outactors
              (Default|EnableInput _array_element)
              (bind _outactors_2 (Actor|GetAllActorsOfClass "/Game/Blueprints/Camera/BP_CharacterSelectCamera.BP_CharacterSelectCamera_C"))
              (for _array_element_2 _outactors_2
                (Game|Player|SetViewTargetwithBlend (Game|GetPlayerController 0) _array_element_2 0.0 "VTBlend_Linear" 0.0 false)
                (Sequencer|Player|Play (Variables|/Script/LevelSequence.LevelSequenceActor|GetSequencePlayer (Variables|Default|GetCinematicStartPlay)) :!class /Script/MovieScene.MovieSceneSequencePlayer))))
          (:1
            (Variables|Default|SetIsInMainMenu false)
            (Sequencer|Player|Play (Variables|/Script/LevelSequence.LevelSequenceActor|GetSequencePlayer (Variables|Default|GetCinematicToControls)) :!class /Script/MovieScene.MovieSceneSequencePlayer))
          (:2
            (Variables|Default|SetIsInMainMenu false)
            (Sequencer|Player|Play (Variables|/Script/LevelSequence.LevelSequenceActor|GetSequencePlayer (Variables|Default|GetCinematiccToOptions)) :!class /Script/MovieScene.MovieSceneSequencePlayer)
            (Variables|Default|SetIsInOption true)
            (Variables|Default|SetCurrentOptionMenu 0))
          (:3
            (Game|QuitGame 0 "Quit")))))))

(event Input|ActionEvents|InputActionNextCharacter
  (params (Key :type Key%20Structure))
  ;[1 1 1] MenuOptions left right
  (:Pressed
    (if (Variables|Default|GetIsInOption)
      (bind _asbp_can_die_rush_game_mode (Utilities|Casting|CastToBP_CanDieRushGameMode (Game|GetGameMode)))
      (switch int (Variables|Default|GetCurrentOptionMenu)
        (:0
          (Variables|/Game/Blueprints/GameModes/BP_CanDieRushGameMode.BP_CanDieRushGameMode_C|SetMaster%20Volume _asbp_can_die_rush_game_mode (Math|Float|Clamp(Float) (+ (Variables|/Game/Blueprints/GameModes/BP_CanDieRushGameMode.BP_CanDieRushGameMode_C|GetMaster%20Volume _asbp_can_die_rush_game_mode) "0.1f") 0.01)))
        (:1
          (Variables|/Game/Blueprints/GameModes/BP_CanDieRushGameMode.BP_CanDieRushGameMode_C|SetSound%20Volume _asbp_can_die_rush_game_mode (Math|Float|Clamp(Float) (+ (Variables|/Game/Blueprints/GameModes/BP_CanDieRushGameMode.BP_CanDieRushGameMode_C|GetSound%20Volume _asbp_can_die_rush_game_mode) "0.1f") 0.01))))
      (Default|ChangeVolume _asbp_can_die_rush_game_mode)
      (bind _asbp_can_die_rush_game_mode_2 (Utilities|Casting|CastToBP_CanDieRushGameMode (Game|GetGameMode)))
      (Audio|SpawnSound2D "/Game/art_assets/SoundEffects/BlackBoard.BlackBoard" (Math|Float|Clamp(Float) (Variables|/Game/Blueprints/GameModes/BP_CanDieRushGameMode.BP_CanDieRushGameMode_C|GetMaster%20Volume _asbp_can_die_rush_game_mode_2) "0.01f" (Variables|/Game/Blueprints/GameModes/BP_CanDieRushGameMode.BP_CanDieRushGameMode_C|GetMaster%20Volume _asbp_can_die_rush_game_mode_2))))))

(event Input|ActionEvents|InputActionPreviousCharacter
  (params (Key :type Key%20Structure))
  ;[1 1 1] MenuOptions left right
  (:Pressed
    (if (Variables|Default|GetIsInOption)
      (bind _asbp_can_die_rush_game_mode (Utilities|Casting|CastToBP_CanDieRushGameMode (Game|GetGameMode)))
      (switch int (Variables|Default|GetCurrentOptionMenu)
        (:0
          (Variables|/Game/Blueprints/GameModes/BP_CanDieRushGameMode.BP_CanDieRushGameMode_C|SetMaster%20Volume _asbp_can_die_rush_game_mode (Math|Float|Clamp(Float) (+ (Variables|/Game/Blueprints/GameModes/BP_CanDieRushGameMode.BP_CanDieRushGameMode_C|GetMaster%20Volume _asbp_can_die_rush_game_mode) "-0.1f") 0.01)))
        (:1
          (Variables|/Game/Blueprints/GameModes/BP_CanDieRushGameMode.BP_CanDieRushGameMode_C|SetSound%20Volume _asbp_can_die_rush_game_mode (Math|Float|Clamp(Float) (+ (Variables|/Game/Blueprints/GameModes/BP_CanDieRushGameMode.BP_CanDieRushGameMode_C|GetSound%20Volume _asbp_can_die_rush_game_mode) "-0.1f") 0.01))))
      (Default|ChangeVolume _asbp_can_die_rush_game_mode)
      (bind _asbp_can_die_rush_game_mode_2 (Utilities|Casting|CastToBP_CanDieRushGameMode (Game|GetGameMode)))
      (Audio|SpawnSound2D "/Game/art_assets/SoundEffects/BlackBoard.BlackBoard" (Math|Float|Clamp(Float) (Variables|/Game/Blueprints/GameModes/BP_CanDieRushGameMode.BP_CanDieRushGameMode_C|GetMaster%20Volume _asbp_can_die_rush_game_mode_2) "0.01f" (Variables|/Game/Blueprints/GameModes/BP_CanDieRushGameMode.BP_CanDieRushGameMode_C|GetMaster%20Volume _asbp_can_die_rush_game_mode_2))))))

(fn ConstructionScript)