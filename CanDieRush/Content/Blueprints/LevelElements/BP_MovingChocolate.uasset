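; BP_MovingChocolate is a level element that rocks a chocolate static mesh back and forth like a constant-speed pendulum.
; BeginPlay picks a random starting angle within a range slightly narrower than MaxAngle, so instances swing out of phase.
; Tick advances the angle by RotationSpeed, applies it as mesh pitch at a fixed yaw, and flips the speed's sign slightly beyond MaxAngle on either side.
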(event EventBeginPlay
  (Variables|Default|SetCurrentAngle (Math|Random|RandomFloatinRange (* (- (Variables|Default|GetMaxAngle) 5.0) -1.0) (- (Variables|Default|GetMaxAngle) 5.0))))

(event Collision|EventActorBeginOverlap
  (params (OtherActor :type Actor%20Object%20Reference)))

(event EventTick
  (params (DeltaSeconds :type Float%20%28single-precision%29))
  (bind _output_get (Variables|Default|SetCurrentAngle (+ (* DeltaSeconds (Variables|Default|GetRotationSpeed)) (Variables|Default|GetCurrentAngle))))
  (Transformation|SetRelativeRotation (Variables|Default|GetStaticMeshComponent01) (Math|Rotator|MakeRotator 0.0 _output_get 9e+01) false false)
  (if (or (>= (Variables|Default|GetCurrentAngle) (+ (Variables|Default|GetMaxAngle) 5.0)) (<= (Variables|Default|GetCurrentAngle) (* (+ (Variables|Default|GetMaxAngle) 5.0) -1.0)))
    (Variables|Default|SetRotationSpeed (* (Variables|Default|GetRotationSpeed) -1.0))))

(fn ConstructionScript)