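; Camera for the trap-building phase that hands over to the race when that phase ends.
; On BeginPlay it sets its start position to the average player spawn location and gathers race characters and waypoints.
; While active, Tick checks whether the camera goal is reached or all building pawns have placed traps, the latter triggering a skip after a short delay.
; It then deactivates and calls the game mode's StartRacingEvent.
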(event EventBeginPlay
  ;[1 1 1] Begin Play
  (Utilities|FlowControl|Sequence
    (:then_0
      ;[1 1 1] Start Pos
      (bind _outactors (Actor|GetAllActorsOfClass "/Game/Blueprints/Player/BP_PlayerSpawn.BP_PlayerSpawn_C"))
      (bind _returnvalue (Class|GameplayStatics|GetActorArrayAverageLocation _outactors))
      (Class|BuildingCameraActor|SetStartPosition _returnvalue))
    (:then_1
      ;[1 1 1] Players
      (bind _outactors_2 (Actor|GetAllActorsOfClass "/Game/Blueprints/Player/BP_RaceCharacter.BP_RaceCharacter_C"))
      (Class|BuildingCameraActor|SetPlayers _outactors_2))
    (:then_2
      ;[1 1 1] WayPoints
      (bind _outactors_3 (Actor|GetAllActorsOfClass "/Game/Blueprints/LevelElements/BP_WayPoint.BP_WayPoint_C"))
      (Class|BuildingCameraActor|SetWayPoints _outactors_3))))

(event Collision|EventActorBeginOverlap
  (params (OtherActor :type Actor%20Object%20Reference)))

(event EventTick
  (params (DeltaSeconds :type Float%20%28single-precision%29))
  (if (Variables|Default|GetIsActive)
    (bind _returnvalue (Class|BuildingCameraActor|BuildCameraGoalReached))
    (if (or _returnvalue (Variables|Default|GetDoSkipBuilding))
      (Development|PrintString "goal reached")
      (Variables|Default|SetIsActive false)
      (bind _asbp_can_die_rush_game_mode (Utilities|Casting|CastToBP_CanDieRushGameMode (Game|GetGameMode)))
      (Default|StartRacingEvent _asbp_can_die_rush_game_mode)
      (goto _label Reset)
      (else
        (Utilities|FlowControl|Sequence
          (:then_0
            (Utilities|FlowControl|DoOnce false :!label _label
              (:Completed
                (bind _outactors (Actor|GetAllActorsOfClass "/Game/Blueprints/Player/BP_BuildingPawn.BP_BuildingPawn_C"))
                (Variables|Default|SetPawns _outactors))))
          (:then_1
            (Variables|Default|SetHasNotPlacedTrap false)
            (for _array_element (Variables|Default|GetPawns)
              (bind _returnvalue_2 (Class|BuildingPawn|HasPlacedTrap _array_element))
              (Variables|Default|SetHasNotPlacedTrap (or (not _returnvalue_2) (Variables|Default|GetHasNotPlacedTrap))))
            (if (or (not (Variables|Default|GetHasNotPlacedTrap)) (Variables|Default|GetDoSkipBuilding))
              (Utilities|FlowControl|Delay 1.0)
              (Variables|Default|SetDoSkipBuilding true))))))))

(fn ConstructionScript)