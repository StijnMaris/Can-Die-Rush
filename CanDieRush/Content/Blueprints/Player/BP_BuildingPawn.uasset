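; Player pawn for the trap-building phase that previews and places one randomly chosen spike, fire or boulder trap.
; BeginPlay picks the trap class and mesh, creates a color-tintable dynamic material and links the pawn to BP_BuildingCamera.
; Placing registers the trap with RacePlayerController and greys the preview.
; Tick clamps the pawn to a rectangle around the camera, and SkipBuilding input sets the camera's skip flag.
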(event EventBeginPlay
  (bind _ourvisiblecomponent (Variables|Default|GetOurVisibleComponent))
  (bind _output_get (Variables|Default|SetRandomInt (Math|Random|RandomInteger 3)))
  (switch int _output_get
    (:Default
      (Variables|Default|SetTrapToSpawn "/Game/Traps/BP_SpikeTrap.BP_SpikeTrap_C" :!label _label)
      (Components|StaticMesh|SetStaticMesh (Variables|Default|GetOurVisibleComponent) "/Game/art_assets/traps/Spikes/MS_Spikes_ondergrond_spekjes.MS_Spikes_ondergrond_spekjes"))
    (:0
      (goto _label))
    (:1
      (Variables|Default|SetTrapToSpawn "/Game/Traps/BP_FireTrap.BP_FireTrap_C")
      (Components|StaticMesh|SetStaticMesh (Variables|Default|GetOurVisibleComponent) "/Game/art_assets/traps/fire/firetrap.firetrap"))
    (:2
      (Variables|Default|SetTrapToSpawn "/Game/Traps/BP_BoulderTrap.BP_BoulderTrap_C")
      (Components|StaticMesh|SetStaticMesh (Variables|Default|GetOurVisibleComponent) "/Game/art_assets/traps/boulder/boulder_full.boulder_full")
      (Transformation|SetWorldScale3D (Variables|Default|GetOurVisibleComponent) "0.250000,0.250000,0.250000")))
  (bind _returnvalue (Rendering|Material|CreateDynamicMaterialInstance _ourvisiblecomponent 0 (Rendering|Material|GetMaterial _ourvisiblecomponent 0) :!class /Script/Engine.PrimitiveComponent))
  (Variables|Default|SetMaterialInst _returnvalue)
  (Rendering|Material|SetVectorParameterValue _returnvalue "Color" "(R=1.000000,G=0.000000,B=0.000000,A=1.000000)" :!class /Script/Engine.MaterialInstanceDynamic)
  (bind _outactors (Actor|GetAllActorsOfClass "/Game/Blueprints/Camera/BP_BuildingCamera.BP_BuildingCamera_C"))
  (for _array_element _outactors
    (Class|BuildingPawn|SetCameratoFollow _array_element)
    (Transformation|SetWorldScale3D (Variables|Transformation|GetRootComponent) "2.000000,2.000000,2.000000")))

(event Collision|EventActorBeginOverlap
  (params (OtherActor :type Actor%20Object%20Reference)))

(event EventTick
  (params (DeltaSeconds :type Float%20%28single-precision%29))
  (bind _ourvisiblecomponent (Variables|Default|GetOurVisibleComponent))
  (bind _returnvalue (Transformation|GetWorldLocation _ourvisiblecomponent))
  (bind (_x _y) (Math|Vector|BreakVector _returnvalue))
  ;[1 1 1] Tick
  (bind _outactors (Actor|GetAllActorsOfClass "/Game/Blueprints/Camera/BP_BuildingCamera.BP_BuildingCamera_C"))
  (for _array_element _outactors
    (Variables|Default|SetCameraX (.X (Math|Vector|BreakVector (Transformation|GetActorLocation _array_element))))
    (Variables|Default|SetCameraY (.Y (Math|Vector|BreakVector (Transformation|GetActorLocation _array_element))))
    (if (or (or (or (< _x (- (Variables|Default|GetCameraX) 1.6e+03)) (> _x (+ (Variables|Default|GetCameraX) 1.6e+03))) (< _y (- (Variables|Default|GetCameraY) 1e+03))) (> _y (+ (Variables|Default|GetCameraY) 1e+03)))
      (Class|BuildingPawn|SetSpawnLocation (Math|Vector|MakeVector (Math|Float|Clamp(Float) _x (- (Variables|Default|GetCameraX) 1.6e+03) (+ (Variables|Default|GetCameraX) 1.6e+03)) (Math|Float|Clamp(Float) _y (- (Variables|Default|GetCameraY) 1e+03) (+ (Variables|Default|GetCameraY) 1e+03)) 0.0)))))

(event Input|ActionEvents|InputActionPlaceTrap
  (params (Key :type Key%20Structure))
  ;[1 1 1] Place Trap
  (:Pressed
    (bind _returnvalue (Class|BuildingPawn|PlaceRandomTrap (Variables|Default|GetTrapToSpawn)))
    (Utilities|IsValid _returnvalue
      (:Is%20Valid
        (bind _asrace_player_controller (Utilities|Casting|CastToRacePlayerController (Pawn|GetController self)))
        (Class|RacePlayerController|AddTrap _asrace_player_controller _returnvalue)
        (CallFunction|SetPawnColorfromColor (Math|Color|MakeColor 50 50 50 255))))))

(event Input|ActionEvents|InputActionSkipBuilding
  (params (Key :type Key%20Structure))
  ;[1 1 1] Skip Building Mode
  (:Pressed
    (bind _outactors (Actor|GetAllActorsOfClass "/Game/Blueprints/Camera/BP_BuildingCamera.BP_BuildingCamera_C"))
    (for _array_element _outactors
      (Variables|/Game/Blueprints/Camera/BP_BuildingCamera.BP_BuildingCamera_C|SetDoSkipBuilding _array_element true))))

(fn ConstructionScript)

(fn SetPawnColorfromController
  (bind _asrace_player_controller (Utilities|Casting|CastToRacePlayerController (Pawn|GetController)))
  (bind _returnvalue (Class|RacePlayerController|GetPlayerColor _asrace_player_controller))
  (Rendering|Material|SetVectorParameterValue (Variables|Default|GetMaterialInst) "Color" (Math|Conversions|ToLinearColor(Color) _returnvalue) :!class /Script/Engine.MaterialInstanceDynamic))

(fn SetPawnColorfromColor
  (params (NewColor :type Color%20Structure))
  (Rendering|Material|SetVectorParameterValue (Variables|Default|GetMaterialInst) "Color" (Math|Conversions|ToLinearColor(Color) NewColor) :!class /Script/Engine.MaterialInstanceDynamic))